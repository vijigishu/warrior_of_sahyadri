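; Damage system component that tracks an actor's health, death, blocking, invincibility and interruptibility.
; Takedamage uses a CanBeDamaged macro to route hits to block, damage or no-damage, following flags in the damage info.
; It fires dispatchers for blocks, death and interrupting damage responses, and returns false on wired exits.
; Heal writes current health plus the amount, clamped to a hardcoded range, into Maxhealth rather than Currenthealth.
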(fn `heal`
  (params (amount :type "Float (double-precision)"))
  (returns (newhealth :type "Float (double-precision)"))
  (if (not (`self.isdead`))
    (bind _output_get (set `self.maxhealth` (`KismetMathLibrary.FClamp` (+ amount (`self.currenthealth`)) 0.0 50.0)))
    (return _output_get)))

(fn `takedamage`
  (params (Damageinfo :type "/Game/Damage_system/takedamage Structure"))
  (returns (wasdamaged :type Boolean))
  (bind (_amount _damage_type _damageresponse _should_damage_invincible _canbeparried _canbeblocked _shouldforceinterrupt) (break `/Game/Damage_system/takedamage` Damageinfo))
  (`self.can be damaged` _should_damage_invincible _canbeblocked
    (:`block damage`
      (`self.onblocked` _canbeparried)
      (return false))
    (:`do damage`
      (bind _output_get (set `self.currenthealth` (- (`self.currenthealth`) _amount)))
      (if (<= _output_get 0.0)
        (set `self.isdead` true)
        (`self.ondeath`)
        (return false)
        (elif (or (`self.isinteruptible`) _shouldforceinterrupt)
          (`self.ondamageresponse` _damageresponse)
          (return false))))
    (:`no damage`
      (return false))))